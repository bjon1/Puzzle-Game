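; Interactable gun pickup that fires bullets and has a telekinesis grab for physics objects.
; Interacting hands it to the player, and SetGunState toggles physics and collision between Dropped and Equipped.
; Fire spawns BP_Bullet at the AmmoSocket, aimed at a distant point along the camera's forward.
; Telekinesis traces from the barrel and grabs via a PhysicsHandle that follows the Arrow each tick; Retract is empty and release logic is unconnected.
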(event `self.ReceiveBeginPlay`
  (`self.SetGunState` "NewEnumerator0"))

(event `/Game/BranMan/BranMan^2/Blueprints/items/InteractionInterface.OnInteracted`
  (params (Player :type "/Game/ThirdPersonBP/Blueprints/ThirdPersonCharacter Object Reference"))
  ;[1 1 1] Pick up gun when E is pressed
  (`/Game/ThirdPersonBP/Blueprints/ThirdPersonCharacter.PickUpGun` Player self)
  (`self.SetGunState` "NewEnumerator1"))

(event `self.ReceiveTick`
  (params (DeltaSeconds :type "Float (single-precision)"))
  ;[1 1 1] Call event tick for arrow - Jeiss
  (`PhysicsHandleComponent.SetTargetLocation` (`self.PhysicsHandle`) (`SceneComponent.K2_GetComponentLocation` (`self.Arrow`))))

(event `Telekinesis`
  (bind _barrel (`self.Barrel`))
  (bind _returnvalue (`SceneComponent.K2_GetComponentLocation` _barrel))
  ;[1 1 1] Telekinesis - Jeiss
  (bind (_outhit _returnvalue_2) (`KismetSystemLibrary.LineTraceSingle` :`Start` _returnvalue :`End` (+ _returnvalue (* (`SceneComponent.GetForwardVector` _barrel) 1000.0)) :`TraceChannel` "TraceTypeQuery1" :`DrawDebugType` "Persistent"))
  (if _returnvalue_2
    (bind (_bblockinghit _binitialoverlap _time _distance _location _impactpoint _normal _impactnormal _physmat _hitactor _hitcomponent) (`GameplayStatics.BreakHitResult` _outhit))
    (if (`SceneComponent.IsSimulatingPhysics` _hitcomponent "None")
      (set `self.isHolding?` true)
      (`PhysicsHandleComponent.GrabComponentAtLocation` (`self.PhysicsHandle`) _hitcomponent "None" (`SceneComponent.K2_GetComponentLocation` _hitcomponent)))))

(fn `Drop`
  (`self.SetGunState` "NewEnumerator0"))

(fn `Fire`
  (params (PlayerCamera :type "CameraComponent Object Reference"))
  (bind _returnvalue (`SceneComponent.GetSocketLocation` (`self.SkeletalMesh`) "AmmoSocket"))
  ;[1 1 1] Fires bullet from ammoSocket, sets direction and velocity based on camera
  (`|SpawnActorFromClass` "/Game/BranMan/BranMan^2/Blueprints/Bullet/BP_Bullet.BP_Bullet_C" (`KismetMathLibrary.MakeTransform` _returnvalue) "Undefined" "OverrideRootScale" null (* (`KismetMathLibrary.Normal` (- (+ (`SceneComponent.K2_GetComponentLocation` PlayerCamera) (* (`SceneComponent.GetForwardVector` PlayerCamera) 10000.0)) _returnvalue)) 5000.0) null))

(fn `GetInteractionText`
  (returns (Text :type Text))
  (return "Pick Up"))

(fn `GetInteractionTextAttach`
  (returns (AttachComponent :type "SceneComponent Object Reference"))
  (return (`self.SkeletalMesh`)))

(fn `Retract`
  ;[1 1 1] Telekinesis - Jeiss
)

(fn `SetGunState`
  (params (gunState :type "/Game/BranMan/BranMan^2/Blueprints/items/Guns/EGunState Enum" :default "NewEnumerator0"))
  (bind _skeletalmesh (`self.SkeletalMesh`))
  ;[1 1 1] Changes gun states depending on if multiple guns are in use
  (bind _output_get (set `self.Gun State` gunState))
  (switch `/Game/BranMan/BranMan^2/Blueprints/items/Guns/EGunState` _output_get
    (:`NewEnumerator0`
      (`PrimitiveComponent.SetCollisionProfileName` (`self.Sphere`) "OverlapAllDynamic" true)
      (`PrimitiveComponent.SetSimulatePhysics` (`self.SkeletalMesh`) true)
      (`PrimitiveComponent.SetCollisionProfileName` (`self.SkeletalMesh`) "DroppedGun" true))
    (:`NewEnumerator1`
      (`PrimitiveComponent.SetCollisionProfileName` (`self.Sphere`) "NoCollision" true)
      (`PrimitiveComponent.SetSimulatePhysics` _skeletalmesh false)
      (`PrimitiveComponent.SetCollisionProfileName` _skeletalmesh "NoCollision" true)
      (`SceneComponent.ResetRelativeTransform` (`self.SkeletalMesh`)))))

(fn `UserConstructionScript`
  (`parent.UserConstructionScript`))