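; BP_BatteryHolder is a socket that accepts a battery and opens a linked battery door.
; Its energy core mesh stays hidden until a BP_Battery actor overlaps the box trigger.
; The overlap then reveals the core, destroys the battery actor, plays a click sound at the core and sets Attached.
; It then calls ActivateDoor on the referenced BPBatteryDoor.
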(event `self.Box.OnComponentBeginOverlap`
  (params (OverlappedComponent :type "PrimitiveComponent Object Reference") (OtherActor :type "Actor Object Reference") (OtherComp :type "PrimitiveComponent Object Reference") (OtherBodyIndex :type Integer) (bFromSweep :type Boolean) (SweepResult :type "HitResult Structure (by ref)"))
  ;[1 1 1] Hides Energy Core until Interacted on -  Jeiss
  ;;[1 1 1] If the overlapped component is a battery...
  (if (== (`GameplayStatics.GetObjectClass` OtherActor) "/Game/Jeiss/BatteryHolder/Meshes/BP_Battery.BP_Battery_C")
    (`|ExecutionSequence`
      (:`then_0`
        ;;[1 1 1] Open the door, show a battery attached on the holder, and remove the battery that just touched the holder - Ben
        (`SceneComponent.SetHiddenInGame` (`self.SM_EnergyCore_A`) false false)
        (`self.K2_DestroyActor` OtherActor)
        (`self.playSound`)
        (set `self.attached` true))
      (:`then_1`
        (`/Game/Jeiss/BatteryHolder/Meshes/BP_BatteryDoor.Activate_door` (`self.BP_BatteryDoor`))))))

(fn `playSound`
  ;[1 1 1] Sound Effect for Battery - Jeiss
  (`GameplayStatics.PlaySoundAtLocation` "/Engine/VREditor/Sounds/UI/Click_on_Button_Cue.Click_on_Button_Cue" (`SceneComponent.K2_GetComponentLocation` (`self.SM_EnergyCore_A`)) (struct) 1.0 1.0 0.0 null null null))

(fn `UserConstructionScript`)